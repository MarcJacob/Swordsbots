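; Interactable map element that serves as the gate to the boss fight.
; On BeginPlay it listens for its room assignment, then binds to that room's cleared delegate to enable interaction.
; Interacting asks the playthrough game subsystem to generate and teleport to the boss arena, then disables further interaction.
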(event EventOnInteraction
  (params (UserController :type Controller%20Object%20Reference) (User :type Actor%20Object%20Reference) (UserToInteractable :type Hit%20Result%20Structure%20%28by%20ref%29))
  (Class|PlaythroughGameSubsystem|GenerateandTeleporttoBossArena (Subsystems|GetPlaythroughGameSubsystem))
  (Variables|Default|SetbCanInteract false))

(event EventBeginPlay
  (EventDispatchers|BindEventtoRoomAssignedDelegate (EventDispatchers|CreateEvent :!event OnRoomAssigned)))

(fn ConstructionScript)

(fn OnRoomAssigned
  (params (AssignedRoom :type Room%20Level%20Object%20Reference))
  (EventDispatchers|BindEventtoOnClearedDelegate AssignedRoom (EventDispatchers|CreateEvent :!event OnRoomCleared)))

(fn OnRoomCleared
  (Variables|Default|SetbCanInteract true))