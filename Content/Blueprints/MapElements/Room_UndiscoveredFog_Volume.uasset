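; Fog volume that covers an undiscovered room and changes appearance as that room is activated and cleared.
; AssignRoom binds to the room's activated and cleared delegates, and construction creates a dynamic material on the volume mesh.
; Activation tints the fog red and sets a new target transparency, while clearing targets full transparency and disables actor collision.
; Tick continuously eases the material's transparency toward its target with a slow delta-time lerp.
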(event EventBeginPlay)

(event Collision|EventActorBeginOverlap
  (params (OtherActor :type Actor%20Object%20Reference)))

(event EventTick
  (params (DeltaSeconds :type Float%20%28single-precision%29))
  (bind _output_get (Variables|Default|SetTransparency (Math|Float|Lerp (Variables|Default|GetTransparency) (Variables|Default|GetTargetTransparency) (/ DeltaSeconds 7.0))))
  (Rendering|Material|SetScalarParameterValue (Variables|Default|GetMaterialInstance) "Transparency" _output_get :!class /Script/Engine.MaterialInstanceDynamic))

(fn ConstructionScript
  (bind _volume_visual (Variables|Default|GetVolume_Visual))
  (bind _returnvalue (Rendering|Material|CreateDynamicMaterialInstance _volume_visual 0 (Rendering|Material|GetMaterial (Variables|Default|GetVolume_Visual) 0) "None" :!class /Script/Engine.PrimitiveComponent))
  (bind _output_get (Variables|Default|SetMaterialInstance _returnvalue))
  (Rendering|Material|SetMaterial _volume_visual 0 _output_get))

(fn AssignedRoomActivated
  (Variables|Default|SetTargetTransparency 0.2)
  (Rendering|Material|SetVectorParameterValue (Variables|Default|GetMaterialInstance) "Color" (Math|Color|MakeColor 1.0 0.0 0.0) :!class /Script/Engine.MaterialInstanceDynamic))

(fn AssignedRoomCleared
  (Variables|Default|SetTargetTransparency 1.0)
  (Collision|SetActorEnableCollision false))

(fn AssignRoom
  (params (AssignedRoom :type Room%20Level%20Object%20Reference))
  (EventDispatchers|BindEventtoOnActivatedDelegate AssignedRoom (EventDispatchers|CreateEvent :!event AssignedRoomActivated))
  (EventDispatchers|BindEventtoOnClearedDelegate AssignedRoom (EventDispatchers|CreateEvent :!event AssignedRoomCleared)))