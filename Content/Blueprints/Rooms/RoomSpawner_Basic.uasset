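; RoomSpawner_Basic is a room spawner Blueprint that links its entry and fog volumes to the room-spawned event.
; On BeginPlay it runs the parent logic, then casts the EntryVolume child actor to RoomActivator and the OcclusionVolume child actor to Room_UndiscoveredFog_Volume.
; Each successful cast leads to an event binding on the RoomSpawned delegate.
; Tick, overlap and the construction script are empty.
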(event EventBeginPlay
  (|CallParentFunction)
  (Utilities|FlowControl|Sequence
    (:then_0
      (bind _asroom_activator (Utilities|Casting|CastToRoomActivator (Variables|/Script/Engine.ChildActorComponent|GetChildActor (Variables|Default|GetEntryVolume))))
      (EventDispatchers|BindEventtoRoomSpawnedDelegate (EventDispatchers|CreateEvent _asroom_activator :!event AssignRoom)))
    (:then_1
      (bind _asroom_undiscovered_fog_volume (Utilities|Casting|CastToRoom_UndiscoveredFog_Volume (Variables|/Script/Engine.ChildActorComponent|GetChildActor (Variables|Default|GetOcclusionVolume))))
      (EventDispatchers|BindEventtoRoomSpawnedDelegate (EventDispatchers|CreateEvent _asroom_undiscovered_fog_volume :!event AssignRoom)))))

(event Collision|EventActorBeginOverlap
  (params (OtherActor :type Actor%20Object%20Reference)))

(event EventTick
  (params (DeltaSeconds :type Float%20%28single-precision%29)))

(fn ConstructionScript)